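; BP_Sound_Potion is a potion actor that reacts to hard impacts with sound and a light flash.
; A component hit with upward normal impulse above a threshold plays attenuated glass and spell-cast sounds at the potion and sets its point light to high intensity.
; While the light is lit, Tick decrements an integer counter and writes it to the intensity.
; The hit event does not reset that counter.
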(event OnComponentHit(Potion)
  (params (HitComponent :type Primitive%20Component%20Object%20Reference) (OtherActor :type Actor%20Object%20Reference) (OtherComp :type Primitive%20Component%20Object%20Reference) (NormalImpulse :type Vector :default "0, 0, 0") (Hit :type Hit%20Result%20Structure%20%28by%20ref%29))
  (bind _potion (Variables|Default|GetPotion))
  (bind _returnvalue (Transformation|GetWorldLocation _potion))
  (if (> (.z NormalImpulse) 1e+03)
    (Audio|PlaySoundatLocation "/Game/Audio/Glass_hit_with_spoon_-_Free_Sound_Effect.Glass_hit_with_spoon_-_Free_Sound_Effect" _returnvalue "0, 0, 0" 1.0 1.0 0.0 "/Game/Audio/NewSoundAttenuation.NewSoundAttenuation" 0 0 0)
    (Audio|PlaySoundatLocation "/Game/Audio/Morrowind_Spell_Cast_Sound_Effect.Morrowind_Spell_Cast_Sound_Effect" _returnvalue "0, 0, 0" 1.0 1.0 0.0 "/Game/Audio/NewSoundAttenuation.NewSoundAttenuation" 0 0 0)
    (Rendering|Components|Light|SetIntensity (Variables|Default|GetPointLight) 8e+03)))

(event EventTick
  (params (DeltaSeconds :type Float%20%28single-precision%29))
  (if (> (Variables|/Script/Engine.LightComponentBase|GetIntensity (Variables|Default|GetPointLight)) 0.0)
    (bind _result (Math|Integer|DecrementInt (Variables|Default|GetIntDecre))
      (:%20%20
        (Rendering|Components|Light|SetIntensity (Variables|Default|GetPointLight) (Math|Conversions|ToFloat(Integer) _result))))))

(fn ConstructionScript)