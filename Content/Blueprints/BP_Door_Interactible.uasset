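; BP_Door_Interactible is a two-mesh door that toggles between open and closed each time its OpenDoor event is called.
; The DoorClose flag selects whether the TL_DoorMouving timeline plays forward or reverses.
; Each timeline update scales the DoorRotation track into a relative yaw for both door meshes.
; An audio component plays whenever the timeline finishes.
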(event Custom|OpenDoor
  (if (Variables|Default|GetDoor_Close)
    (Variables|Default|SetDoor_Close false)
    (bind _door_rotation (Timeline|TL_DoorMouving Play)
      (:Update
        (bind _result (Math|Float|NegateFloat (* _door_rotation 8e+01))
          (:%20%20
            (Transformation|SetRelativeRotation (Variables|Default|GetDoor_3_StaticMeshComponent0) (Math|Rotator|MakeRotator 0.0 0.0 _result) false false)
            (Transformation|SetRelativeRotation (Variables|Default|GetDoor_4_StaticMeshComponent0) (Math|Rotator|MakeRotator 0.0 0.0 (* _door_rotation 8e+01)) false false))))
      (:Finished
        (Audio|Components|Audio|Play (Variables|Default|GetAudio) 0.0)))
    (else
      (Variables|Default|SetDoor_Close true)
      (Timeline|TL_DoorMouving Reverse))))

(fn ConstructionScript)